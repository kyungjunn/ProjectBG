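; Game mode that spawns randomized loot at BeginPlay for each location in DT_ItemGroupLocation.
; It first caches probability totals and row names for item count, type and per-type IDs, except Weapon and Accessories.
; Each spawned BP_ItemGroup supplies random transforms for a rolled number of distinct item types, each resolved to an ID and spawned as BP_TestItem.
; Rolls use cumulative-weight selection; older array-expansion versions remain disconnected.
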(event EventBeginPlay
  (CallFunction|GenerateItems))

(event EventTick
  (params (DeltaSeconds :type Float%20%28single-precision%29)))

(fn ConstructionScript)

(fn GenerateItems
  ;[0.15 0.15 0.15 0.5] 필요한 모든 아이템 데이터 테이블 가져오기
  (|CollapseGraph
    (:OutExecute
      ;[0.15 0.15 0.15 0.5] data table의 전체 로우 네임 가져오기
      (bind _outrownames (DataTable|GetDataTableRowNames "/Game/Blueprints/Datas/DataTable/ItemGeneration/DT_ItemGroupLocation.DT_ItemGroupLocation"))
      (for _array_element _outrownames
        (bind _returnvalue (Utilities|GetDataTableRow "/Game/Blueprints/Datas/DataTable/ItemGeneration/DT_ItemGroupLocation.DT_ItemGroupLocation" _array_element)
          (:then
            (bind _returnvalue_2 (Game|SpawnActorfromClass "/Game/Blueprints/Items/BP_ItemGroup.BP_ItemGroup_C" (Math|Transform|MakeTransform (.location _returnvalue) "0, 0, 0" "1.000000,1.000000,1.000000") "Undefined" "MultiplyWithRoot" 0 0))
            (LocalVariables|SetItemGroupRef _returnvalue_2)
            ;[0.15 0.15 0.15 0.5] 초기화
            (Utilities|Array|Clear (LocalVariables|GetItemTypeArr))
            (bind _number (CallFunction|RandomNameNumber (LocalVariables|GetNumberProbabilityInfo)))
            (LocalVariables|SetSpawnTransforms (Default|GetRandomTransforms (LocalVariables|GetItemGroupRef) _number))
            (for _index (range 1 _number)
              ;[0.15 0.15 0.15 0.5] 랜덤 아이템 타입 설정
              (bind _itemtype (CallFunction|RandomItemType (LocalVariables|GetItemTypeProbabilityInfo) :!label _label))
              ;[0.15 0.15 0.15 0.5] 랜덤 아이템끼리 중복 방지
              (if (== (Utilities|Array|FindItem (LocalVariables|GetItemTypeArr) _itemtype) -1)
                (Utilities|Array|Add (LocalVariables|GetItemTypeArr) _itemtype)
                (else
                  (goto _label))))
            (for _array_element_2 (LocalVariables|GetItemTypeArr)
              (bind _spawnitem (CallFunction|RandomItemId (LocalVariables|GetItemIdProbabilityInfos) _array_element_2))
              (Utilities|Array|Add (LocalVariables|GetSpawnItemArr) _spawnitem))
            (for (_array_element_3 _array_index) (LocalVariables|GetSpawnItemArr)
              (LocalVariables|SetItemType (.itemtype _array_element_3))
              (LocalVariables|SetSpawnId (.id _array_element_3))
              (Game|SpawnActorfromClass "/Game/Blueprints/BP_TestItem.BP_TestItem_C" (Utilities|Array|Get(acopy) (LocalVariables|GetSpawnTransforms) _array_index) "Undefined" "MultiplyWithRoot" 0 0))
            (Utilities|Array|Clear (LocalVariables|GetSpawnItemArr))))))))

(fn RandomNameNumber
  (params (NumberProbability :type ST%20Probability%20Info%20Structure))
  ;[0.15 0.15 0.15 0.5] 가중치 누적 랜덤 방식 -> 위와 같은 로직이어도 더 짧은 순회만으로 구현 => 메모리 아낌.
  (LocalVariables|SetRandomValue (Math|Random|RandomIntegerinRange 1 (.totalpercent NumberProbability)))
  ;;[0.15 0.15 0.15 0.5] 총 3회 순회
  (for _array_element (.rownames NumberProbability)
    (bind _returnvalue (Utilities|GetDataTableRow "/Game/Blueprints/Datas/DataTable/ItemGeneration/DT_NumberProbabilitys.DT_NumberProbabilitys" _array_element)
      (:then
        ;;[0.15 0.15 0.15 0.5] 여기도 최종 100
        (bind _output_get (LocalVariables|SetSumPercent (+ (LocalVariables|GetSumPercent) (.percent _returnvalue))))
        ;;[0.15 0.15 0.15 0.5] 그 와중에 랜덤한 값보다 크다면?
        (if (>= _output_get (LocalVariables|GetRandomValue))
          (return (.number _returnvalue)))))))

(fn RandomItemType
  (params (ItemTypeProbabilityInfo :type ST%20Probability%20Info%20Structure))
  (LocalVariables|SetRandomValue (Math|Random|RandomIntegerinRange 1 (.totalpercent ItemTypeProbabilityInfo)))
  (for _array_element (.rownames ItemTypeProbabilityInfo)
    (bind _returnvalue (Utilities|GetDataTableRow "/Game/Blueprints/Datas/DataTable/ItemGeneration/DT_ItemTypeProbability.DT_ItemTypeProbability" _array_element)
      (:then
        (bind _output_get (LocalVariables|SetSumPercent (+ (LocalVariables|GetSumPercent) (.percent _returnvalue))))
        (if (>= _output_get (LocalVariables|GetRandomValue))
          (return (.itemtype _returnvalue)))))))

(fn RandomItemId
  (params (ItemProbabilityInfo :type Map%20of%20E_ItemType%20Enums%20to%20Structs :default "NewEnumerator0") (ItemType :type E_ItemType%20Enum :default "NewEnumerator0"))
  (bind _value (Utilities|Map|Find ItemProbabilityInfo ItemType))
  (bind (_totalpercent _rownames) (Utilities|Struct|BreakST_ProbabilityInfo _value))
  (LocalVariables|SetRandomValue (Math|Random|RandomIntegerinRange 0 _totalpercent))
  (for _array_element _rownames
    (bind _returnvalue (Utilities|GetDataTableRow (Utilities|Select :Index ItemType :NewEnumerator0 "/Game/Blueprints/Datas/DataTable/ItemGeneration/DT_WeaponProbability.DT_WeaponProbability" :NewEnumerator1 "/Game/Blueprints/Datas/DataTable/ItemGeneration/DT_WeaponAccProbability.DT_WeaponAccProbability" :NewEnumerator2 "/Game/Blueprints/Datas/DataTable/ItemGeneration/DT_AmmoProbability.DT_AmmoProbability" :NewEnumerator3 "/Game/Blueprints/Datas/DataTable/ItemGeneration/DT_HealthProbability.DT_HealthProbability" :NewEnumerator4 "/Game/Blueprints/Datas/DataTable/ItemGeneration/DT_BoostProbability.DT_BoostProbability" :NewEnumerator5 "/Game/Blueprints/Datas/DataTable/ItemGeneration/DT_HelmetProbability.DT_HelmetProbability" :NewEnumerator6 "/Game/Blueprints/Datas/DataTable/ItemGeneration/DT_VestProbability.DT_VestProbability" :NewEnumerator7 "/Game/Blueprints/Datas/DataTable/ItemGeneration/DT_BackpackProbability.DT_BackpackProbability") _array_element)
      (:then
        (bind _output_get (LocalVariables|SetSumPercent (+ (LocalVariables|GetSumPercent) (Utilities|Struct|BreakST_ItemProbability _returnvalue))))
        (if (>= _output_get (LocalVariables|GetRandomValue))
          (return (Utilities|Struct|MakeST_SpawnItem ItemType _array_element)))))))