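; MathUtils is a utility Blueprint of rotation helpers that reduce rotations to yaw only, with pitch and roll zeroed.
; GetYawConAActRotation takes a pawn and a pressed flag, returning the control rotation's yaw when pressed and the actor rotation's yaw otherwise.
; GetYawOnlyRotation applies the same flattening to any supplied rotator.
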(fn GetYawConAActRotation
  (params (TargetPawn :type Pawn%20Object%20Reference) (bIsPressed :type Boolean))
  (if bIsPressed
    (return (Math|Rotator|MakeRotator 0.0 0.0 (.yaw (Pawn|GetControlRotation TargetPawn :!class /Script/Engine.Pawn))))
    (else
      (return (Math|Rotator|MakeRotator 0.0 0.0 (.yaw (Transformation|GetActorRotation TargetPawn)))))))

(fn GetYawOnlyRotation
  (params (Rotator :type Rotator))
  (return (Math|Rotator|MakeRotator 0.0 0.0 (.Yaw (Math|Rotator|BreakRotator Rotator)))))